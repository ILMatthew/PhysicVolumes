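; Volume connector Blueprint that shows its open or closed state through a colored DebugOpen component.
; The construction script gives DebugOpen a dynamic instance of M_DebugSimpleColor and tints it green when open, red when closed.
; BeginPlay binds a handler to the connector-opened event, and SetDebugSphere applies the same color switch from its IsOpen argument.
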(event `self.ReceiveBeginPlay`
  (add `self.OnConnectorOpened` (`|CreateDelegate` :!event `SetDebugSphere`)))

(event `SetDebugSphere` :!signature `self.OnConnectorOpened`
  (params (IsOpen :type Boolean))
  (`MeshComponent.SetVectorParameterValueOnMaterials` (`self.DebugOpen`) "Color" (`KismetMathLibrary.Conv_LinearColorToVector` (`KismetMathLibrary.SelectColor` (struct :`R` 0.062223 :`G` 1.0 :`A` 1.0) (struct :`R` 1.0 :`A` 1.0) IsOpen))))

(fn `UserConstructionScript`
  (bind _returnvalue (`KismetMaterialLibrary.CreateDynamicMaterialInstance` "/PhysicVolumes/Materials/M_DebugSimpleColor.M_DebugSimpleColor"))
  (`PrimitiveComponent.SetMaterial` (`self.DebugOpen`) 0 _returnvalue)
  (`MeshComponent.SetVectorParameterValueOnMaterials` (`self.DebugOpen`) "Color" (`KismetMathLibrary.Conv_LinearColorToVector` (`KismetMathLibrary.SelectColor` (struct :`R` 0.062223 :`G` 1.0 :`A` 1.0) (struct :`R` 1.0 :`A` 1.0) (`self.bIsOpen`)))))