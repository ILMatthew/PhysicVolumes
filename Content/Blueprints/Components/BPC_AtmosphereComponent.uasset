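; Actor component that holds atmosphere info (temperature, pressure, air composition) and visualizes it on its owner for debugging.
; On BeginPlay it adds a collisionless sphere mesh to the owner with a dynamic debug color material.
; Each Tick it prints the temperature and tints the sphere from red to green using pressure as the lerp alpha.
; Printouts for air composition and pressure exist but are disconnected.
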(event `self.ReceiveBeginPlay`
  (bind _returnvalue (`|AddComponentByClass` (`self.GetOwner`) "/Script/Engine.StaticMeshComponent" false (`KismetMathLibrary.MakeTransform` (0.0 0.0 0.0))))
  (`StaticMeshComponent.SetStaticMesh` _returnvalue "/Engine/BasicShapes/Sphere.Sphere")
  (bind _returnvalue_2 (`KismetMaterialLibrary.CreateDynamicMaterialInstance` "/PhysicVolumes/Materials/M_DebugSimpleColor.M_DebugSimpleColor"))
  (bind _output_get (set `self.DebugMaterial` _returnvalue_2))
  (`PrimitiveComponent.SetMaterial` _returnvalue 0 _output_get)
  (`PrimitiveComponent.SetCollisionEnabled` _returnvalue "NoCollision"))

(event `self.ReceiveTick`
  (params (DeltaSeconds :type "Float (single-precision)"))
  (bind (_pressure _aircomposition _temperature) (break `AtmosphereInfo` (`self.atmosphereInfo`)))
  (`|ExecutionSequence`
    (:`then_1`
      (`KismetSystemLibrary.PrintString` (`KismetStringLibrary.Concat_StrStr` (`KismetSystemLibrary.GetDisplayName` (`self.GetOwner`)) " temperature: " (`KismetStringLibrary.Conv_DoubleToString` _temperature)) true false (struct :`R` 1.0 :`G` 0.528106 :`A` 1.0) 0.001)
      (`MaterialInstanceDynamic.SetVectorParameterValue` (`self.DebugMaterial`) "Color" (`KismetMathLibrary.LinearColorLerp` (struct :`R` 1.0 :`B` 0.032468 :`A` 1.0) (struct :`R` 0.117366 :`G` 1.0 :`A` 1.0) _pressure)))))