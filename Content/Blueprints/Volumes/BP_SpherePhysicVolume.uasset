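; Spherical physics volume Blueprint whose construction script lays out six debug components that visualize gravity direction.
; It scales each component's relative location by the sphere radius.
; When InheritFromParent is set, it finds overlapping PhysicVolumes with priority exactly one lower and rotates all six components to that volume's gravity direction, sampled using that volume as the simulated object.
; The event graph holds no runtime logic.
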(event `self.ReceiveTick`
  (params (DeltaSeconds :type "Float (single-precision)")))

(fn `UserConstructionScript`
  (bind _debuggravityvector1 (`self.DebugGravityVector1`))
  (bind _debuggravityvector2 (`self.DebugGravityVector2`))
  (bind _debuggravityvector3 (`self.DebugGravityVector3`))
  (bind _debuggravityvector4 (`self.DebugGravityVector4`))
  (bind _debuggravityvector5 (`self.DebugGravityVector5`))
  (bind _debuggravityvector (`self.DebugGravityVector`))
  (`|ExecutionSequence`
    (:`then_0`
      (`SceneComponent.K2_SetRelativeLocation` _debuggravityvector1 (* (`SceneComponent.RelativeLocation` _debuggravityvector1) (`self.SphereRadius`)) false false)
      (`SceneComponent.K2_SetRelativeLocation` _debuggravityvector2 (* (`SceneComponent.RelativeLocation` _debuggravityvector2) (`self.SphereRadius`)) false false)
      (`SceneComponent.K2_SetRelativeLocation` _debuggravityvector3 (* (`SceneComponent.RelativeLocation` _debuggravityvector3) (`self.SphereRadius`)) false false)
      (`SceneComponent.K2_SetRelativeLocation` _debuggravityvector4 (* (`SceneComponent.RelativeLocation` _debuggravityvector4) (`self.SphereRadius`)) false false)
      (`SceneComponent.K2_SetRelativeLocation` _debuggravityvector5 (* (`SceneComponent.RelativeLocation` _debuggravityvector5) (`self.SphereRadius`)) false false)
      (`SceneComponent.K2_SetRelativeLocation` _debuggravityvector (* (`SceneComponent.RelativeLocation` _debuggravityvector) (`self.SphereRadius`)) false false))
    (:`then_1`
      (if (`self.InheritFromParent`)
        (bind _assphere_collision (cast `SphereComponent` (`self.RootComponent`)))
        (bind _outactors (`KismetSystemLibrary.ComponentOverlapActors` _assphere_collision (`self.GetTransform`) (`|MakeArray` "ObjectTypeQuery2" :!type "EObjectTypeQuery Enum") "/Script/PhysicVolumes.PhysicVolume"))
        (for _array_element _outactors
          (bind _asphysic_volume (cast `PhysicVolume` _array_element))
          (if (== (`self.GetPriority` _asphysic_volume) (- (`self.GetPriority`) 1))
            (bind _returnvalue (`KismetMathLibrary.FindLookAtRotation` (`KismetMathLibrary.Vector_Zero`) (`self.GetGravityDirection` _asphysic_volume _asphysic_volume false)))
            (`SceneComponent.K2_SetWorldRotation` _debuggravityvector1 _returnvalue false false)
            (`SceneComponent.K2_SetWorldRotation` _debuggravityvector2 _returnvalue false false)
            (`SceneComponent.K2_SetWorldRotation` _debuggravityvector3 _returnvalue false false)
            (`SceneComponent.K2_SetWorldRotation` _debuggravityvector4 _returnvalue false false)
            (`SceneComponent.K2_SetWorldRotation` _debuggravityvector5 _returnvalue false false)
            (`SceneComponent.K2_SetWorldRotation` _debuggravityvector _returnvalue false false)))))))